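; Chest actor that players open through an Interact interface to access its inventory.
; On BeginPlay it creates a hidden, disabled, centered inventory widget titled "Chest".
; After a short delay it seeds its InventoryBP by spawning a temporary armor actor, picking up its item info, then destroying it.
; Interact passes the chest to the character, which opens the chest and inventory.
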(event EventBeginPlay
  (Utilities|FlowControl|Sequence
    (:then_0
      (bind _returnvalue (UserInterface|CreateWidget "/Game/Inventory/Widgets/InventoryWidget.InventoryWidget_C"))
      (bind _output_get (Variables|Default|SetChestWidgetRef _returnvalue))
      (UserInterface|Viewport|AddtoViewport _output_get 0)
      (Widget|SetIsEnabled _output_get false)
      (Widget|SetVisibility _output_get "Hidden")
      (Class|UserWidget|SetDesiredSizeinViewport _output_get "(X=500.000000,Y=500.000000)")
      (Class|UserWidget|SetAnchorsinViewport _output_get (Utilities|Struct|MakeAnchors "(X=0.500000,Y=0.500000)" "(X=0.500000,Y=0.500000)"))
      (Class|UserWidget|SetAlignmentinViewport _output_get "(X=0.500000,Y=0.500000)")
      (Rendering|Components|TextRender|SetText (Variables|/Game/Inventory/Widgets/InventoryWidget.InventoryWidget_C|GetInventoryName _output_get) "Chest"))
    (:then_1
      (Utilities|FlowControl|Delay 0.2)
      (bind _returnvalue_2 (Game|SpawnActorfromClass "/Game/Inventory/Blueprints/ArmorBase_BP.ArmorBase_BP_C" (Math|Transform|MakeTransform "0, 0, 0" "0, 0, 0" "1,1,1") "Undefined" 0 0))
      (Default|-PickUpItem (Variables|Default|GetInventory_BP) (Variables|/Game/Inventory/ItemBase_BP.ItemBase_BP_C|GetItemInfo _returnvalue_2))
      (Actor|DestroyActor _returnvalue_2))))

(event Collision|EventActorBeginOverlap
  (params (OtherActor :type Actor%20Object%20Reference)))

(event EventTick
  (params (DeltaSeconds :type Float%20%28single-precision%29)))

(event EventInteract
  (params (CharBaseRef :type Character%20Base%20BP%20Object%20Reference))
  ;[1 1 1] Interact inteface
  (bind _output_get (Variables|Default|SetCharBaseRef CharBaseRef))
  (Variables|/Game/Inventory/CharacterBase_BP.CharacterBase_BP_C|SetChestRef _output_get self)
  (Default|-OpenChest (Variables|Default|GetCharBaseRef))
  (Default|-OpenInventory (Variables|Default|GetCharBaseRef)))

(fn ConstructionScript)