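; Inventory component shared by characters and chests, holding item structs in a slot-limited array.
; Picking up rejects one null item type or a full inventory, then creates an item widget in the owning character's main inventory widget or the chest's widget.
; Dropping spawns the item's class at a random horizontal offset around the owner and removes it from the array, while helpers fetch or remove by slot.
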(event EventBeginPlay)

(event EventTick
  (params (DeltaSeconds :type Float%20%28single-precision%29)))

(fn -PickUpItem
  (params (Item :type S%20Item%20Info%20Structure))
  (bind _returnvalue (Components|GetOwner))
  (if (Utilities|Enum|NotEqual(Enum) (.ItemType (Utilities|Struct|BreakS_ItemInfo Item)) "NewEnumerator5")
    (LocalVariables|SetItemInfoToAdd Item)
    (if (< (Utilities|Array|Length (Variables|Default|GetItemsInside)) (Variables|Default|GetAmountOfSlots))
      (Utilities|Array|Add (Variables|Default|GetItemsInside) (LocalVariables|GetItemInfoToAdd))
      ;[1 1 1] Create slot in Char widget
      (bind _ascharacter_base_bp (Utilities|Casting|CastToCharacterBase_BP _returnvalue)
        (:then
          (bind _returnvalue_2 (UserInterface|CreateWidget "/Game/Inventory/Widgets/ItemWidget.ItemWidget_C" 0 true))
          (Rendering|Components|TextRender|SetText (Variables|/Game/Inventory/Widgets/ItemWidget.ItemWidget_C|GetItemName _returnvalue_2) (Utilities|Text|ToText(Name) (.ItemName (Utilities|Struct|BreakS_ItemInfo (LocalVariables|GetItemInfoToAdd)))))
          (Class|VerticalBox|AddChildtoVerticalBox (Variables|/Game/Inventory/Widgets/InventoryWidget.InventoryWidget_C|GetVerticalBox_1 (Variables|/Game/Inventory/Widgets/Main_Widget.Main_Widget_C|GetInventoryWidget (Variables|/Game/Inventory/CharacterBase_BP.CharacterBase_BP_C|GetMainWidgetRef _ascharacter_base_bp))) _returnvalue_2)
          (return true))
        (:CastFailed
          ;[1 1 1] Create slot in Chest widget
          (bind _aschest_bp (Utilities|Casting|CastToChest_BP _returnvalue))
          (bind _returnvalue_3 (UserInterface|CreateWidget "/Game/Inventory/Widgets/ItemWidget.ItemWidget_C"))
          (Rendering|Components|TextRender|SetText (Variables|/Game/Inventory/Widgets/ItemWidget.ItemWidget_C|GetItemName _returnvalue_3) (Utilities|Text|ToText(Name) (.ItemName (Utilities|Struct|BreakS_ItemInfo (LocalVariables|GetItemInfoToAdd)))))
          (Class|VerticalBox|AddChildtoVerticalBox (Variables|/Game/Inventory/Widgets/InventoryWidget.InventoryWidget_C|GetVerticalBox_1 (Variables|/Game/Inventory/Chest_BP.Chest_BP_C|GetChestWidgetRef _aschest_bp)) _returnvalue_3)
          (return true)))
      (else
        (Development|PrintString "Inventory FULL!!!")
        (return false)))
    (else
      (Development|PrintString "Item Null")
      (return false))))

(fn -DropItem
  (params (SlotNumber :type Integer))
  (bind _returnvalue (Math|Random|RandomUnitVector))
  (bind (_x _y) (Math|Vector|BreakVector _returnvalue))
  (Variables|Default|SetSlotNumber SlotNumber)
  (if (!= (Utilities|Array|Length (Variables|Default|GetItemsInside)) 0)
    (Game|SpawnActorfromClass (.ItemClass (Utilities|Struct|BreakS_ItemInfo (Utilities|Array|Get(acopy) (Variables|Default|GetItemsInside) (Variables|Default|GetSlotNumber)))) (Math|Transform|MakeTransform (+ (Transformation|GetActorLocation (Components|GetOwner)) (* (Math|Vector|MakeVector _x _y 0.0) 1e+02)) "0, 0, 0" "1,1,1") "AdjustIfPossibleButAlwaysSpawn" 0 0)
    (Utilities|Array|RemoveIndex (Variables|Default|GetItemsInside) (Variables|Default|GetSlotNumber))
    (else
      (Development|PrintString "Inventory empty"))))

(fn -GetItem
  (params (SlotNumber :type Integer))
  (return (Utilities|Array|Get(acopy) (Variables|Default|GetItemsInside) SlotNumber)))

(fn -RemovefromInv
  (params (ItemSlotNumber :type Integer))
  (Utilities|Array|RemoveIndex (Variables|Default|GetItemsInside) ItemSlotNumber))