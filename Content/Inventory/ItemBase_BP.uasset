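; Base actor for world items that a character can pick up into its inventory.
; The construction script labels the item with its type and packs its properties, object name and class into an ItemInfo struct.
; BeginPlay links the name widget to the item and shows the type.
; The Interact interface event passes ItemInfo to the character's InventoryBP and destroys the actor on success; the local PickUp function only returns false.
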(event EventBeginPlay
  (bind _aswbp_item_name (Utilities|Casting|CastToWBP_ItemName (UserInterface|GetUserWidgetObject (Variables|Default|GetName))))
  (Variables|/Game/Inventory/Widgets/WBP_ItemName.WBP_ItemName_C|SetItemBaseRef _aswbp_item_name self)
  (Rendering|Components|TextRender|SetText (Variables|/Game/Inventory/Widgets/WBP_ItemName.WBP_ItemName_C|GetItemNameText _aswbp_item_name) (Utilities|Text|ToText(String) (Utilities|String|EnumtoString (Variables|Base|GetType)))))

(event Collision|EventActorBeginOverlap
  (params (OtherActor :type Actor%20Object%20Reference)))

(event EventInteract
  (params (CharBaseRef :type Character%20Base%20BP%20Object%20Reference))
  ;[1 1 1] Interact interface
  (bind _success_ (Default|-PickUpItem (Variables|/Game/Inventory/CharacterBase_BP.CharacterBase_BP_C|GetInventory_BP CharBaseRef) (Variables|Default|GetItemInfo)))
  (if _success_
    (Actor|DestroyActor)))

(event EventTick
  (params (DeltaSeconds :type Float%20%28single-precision%29)))

(fn ConstructionScript
  (Rendering|Components|TextRender|SetText (Variables|Default|GetNameR) (Utilities|Text|ToText(String) (Utilities|String|EnumtoString (Variables|Base|GetType))))
  (Variables|Base|SetItemName (Utilities|String|StringToName (Utilities|GetObjectName self)))
  (Variables|Default|SetItemInfo (Utilities|Struct|MakeS_ItemInfo (Variables|Base|GetItemName) (Variables|Base|GetType) (Variables|Base|GetMass) (Variables|Base|GetVolume) (Variables|Base|GetMaterial/Amount) (Variables|Base|GetIsQuest?) 0.0 0.0 (Utilities|Map|MakeMap "NewEnumerator6" 0.0) (Utilities|GetClass self))))

(fn PickUp
  (params (ItemInfo :type S%20Item%20Info%20Structure))
  (return false))